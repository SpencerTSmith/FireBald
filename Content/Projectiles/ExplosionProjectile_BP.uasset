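; Explosion projectile actor that plays an explosion sound at its location and shifts itself upward when spawned.
; On overlap with a Goblin_Character, it casts to Goblin_BP and checks a Goblin variable's IsStunned flag, though that variable is set to None just before the read.
; If the flag is true, the explosion enlarges itself and moves further up; no damage or destruction is handled here.
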(event `self.ReceiveBeginPlay`
  (`GameplayStatics.PlaySoundAtLocation` "/Game/BigFiles/Audio/explosion.explosion" (`self.K2_GetActorLocation`) (struct) 1.0 1.0 0.0 null null null null)
  (`self.K2_AddActorWorldOffset` (0.0 0.0 60.0) false true))

(event `self.ReceiveActorBeginOverlap`
  (params (OtherActor :type "Actor Object Reference"))
  (if (`GameplayStatics.ObjectIsA` OtherActor "/Script/MyProject.Goblin_Character")
    (cast `/Game/Characters/Enemy/Goblin_BP` OtherActor)
    (bind _output_get (set `self.Goblin` null))
    (if (`/Game/Characters/Enemy/Goblin_BP.IsStunned` _output_get)
      (`self.SetActorScale3D` (2.0 2.0 2.0))
      (`self.K2_AddActorWorldOffset` (0.0 0.0 120.0) false true))))

(fn `UserConstructionScript`)