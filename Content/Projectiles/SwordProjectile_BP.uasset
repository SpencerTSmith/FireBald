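; Sword swing projectile that limits how many overlaps a single swing can cleave through.
; It plays the swing sound on BeginPlay, counts MaxCleave down on each actor overlap, and destroys itself once the count drops below zero.
; Every tick it feeds the first player character's velocity to its ProjectileMovementComponent as a local-space velocity, so its motion depends on the player's movement.
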(event `self.ReceiveBeginPlay`
  (`GameplayStatics.PlaySound2D` "/Game/BigFiles/Audio/sword_swing.sword_swing" 1.0 1.0 0.0 null null))

(event `self.ReceiveActorBeginOverlap`
  (params (OtherActor :type "Actor Object Reference"))
  (bind _output_get (set `self.MaxCleave` (- (`self.MaxCleave`) 1)))
  (if (< _output_get 0)
    (`self.K2_DestroyActor`)))

(event `self.ReceiveTick`
  (params (DeltaSeconds :type "Float (single-precision)"))
  (`ProjectileMovementComponent.SetVelocityInLocalSpace` (`self.ProjectileMovementComponent`) (`self.GetVelocity` (`GameplayStatics.GetPlayerCharacter` 0))))

(fn `UserConstructionScript`)