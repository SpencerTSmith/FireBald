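; Enemy character Blueprint that chases the player and reacts to projectile hits.
; When PawnSensing sees a pawn, it sets a seeing flag and issues an AI move toward player character 0.
; On overlap, stun projectiles tint the sprite cyan and disable movement, with no recovery here.
; Sword projectiles subtract health and tint the sprite red, destroying the enemy at zero health.
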(event `self.ReceiveActorBeginOverlap`
  (params (OtherActor :type "Actor Object Reference"))
  ;[1 1 1] Different Attack Recieved Behavior
  (if (`GameplayStatics.ObjectIsA` OtherActor "/Game/Projectiles/StunProjectile_BP.StunProjectile_BP_C")
    (`PaperSpriteComponent.SetSpriteColor` (`self.PaperSprite`) (struct :`G` 0.803862 :`B` 1.0 :`A` 1.0))
    (`CharacterMovementComponent.DisableMovement` (`self.CharacterMovement`))
    (elif (`GameplayStatics.ObjectIsA` OtherActor "/Game/Projectiles/SwordProjectile_BP.SwordProjectile_BP_C")
      (bind _output_get (set `self.Health` (- (`self.Health`) 1.0)))
      (`PaperSpriteComponent.SetSpriteColor` (`self.PaperSprite`) (struct :`R` 1.0 :`B` 0.031996 :`A` 1.0))
      (if (<= _output_get 0.0)
        (`self.K2_DestroyActor`)))))

(event `self.PawnSensing.OnSeePawn`
  (params (Pawn :type "Pawn Object Reference"))
  ;[1 1 1] See and Move to Player
  (set `self.isSeeingPlayer` true)
  (`self.FollowPlayer`))

(event `FollowPlayer`
  ;[1 1 1] See and Move to Player
  (if (`self.isSeeingPlayer`)
    (`|AIMoveTo` self (0.0 0.0 0.0) (`GameplayStatics.GetPlayerCharacter` 0))))

(fn `UserConstructionScript`)