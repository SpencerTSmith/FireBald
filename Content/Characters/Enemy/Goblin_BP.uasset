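; Goblin enemy character that chases the player once PawnSensing spots them, using AI MoveTo.
; Overlap branches on projectile class: stun tints it, freezes movement and swaps to a frozen flipbook until a sword hit re-enables movement.
; Sword hits reduce health and knock it along the player's facing, adding score through GameModeDef on death.
; Fireballs kill instantly without scoring; death sounds use a pitch randomized at BeginPlay.
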(event `self.ReceiveBeginPlay`
  (set `self.DeathPitch` (`KismetMathLibrary.RandomFloatInRange` 1.0 9.0)))

(event `self.ReceiveActorBeginOverlap`
  (params (OtherActor :type "Actor Object Reference"))
  (bind _charactermovement (`self.CharacterMovement`))
  ;[1 1 1] Different Attack Recieved Behavior
  ;;[1 1 1] Stun
  (if (`GameplayStatics.ObjectIsA` OtherActor "/Game/Projectiles/StunProjectile_BP.StunProjectile_BP_C")
    (set `self.IsStunned` true)
    (`PaperFlipbookComponent.SetSpriteColor` (`self.Sprite`) (struct :`G` 0.85423 :`B` 1.0 :`A` 1.0))
    (`ActorComponent.SetActive` _charactermovement false false)
    (`PaperFlipbookComponent.SetFlipbook` (`self.Sprite`) "/Game/BigFiles/Sprites/Enemy/goblin_frozen-Sheet_flip.goblin_frozen-Sheet_flip")
    (`GameplayStatics.PlaySoundAtLocation` "/Game/BigFiles/Audio/freeze.freeze" (`self.K2_GetActorLocation`) (struct) 1.0 1.0 0.0 null null null null)
    (else
      ;;[1 1 1] Sword
      (if (`GameplayStatics.ObjectIsA` OtherActor "/Game/Projectiles/SwordProjectile_BP.SwordProjectile_BP_C")
        (set `self.IsStunned` false)
        (`ActorComponent.SetActive` _charactermovement true false)
        (bind _output_get (set `self.Health` (- (`self.Health`) 1.0)))
        (`PaperFlipbookComponent.SetSpriteColor` (`self.Sprite`) (struct :`R` 1.0 :`B` 0.014804 :`A` 1.0))
        (`GameplayStatics.PlaySound2D` "/Game/BigFiles/Audio/impact.impact" 1.0 1.0 0.0 null null)
        (if (<= _output_get 0.0)
          (`self.DeathSound`)
          (`self.K2_DestroyActor`)
          (bind _asgame_mode_def (cast `/Game/Core/GameModeDef` (`GameplayStatics.GetGameMode`)))
          (`/Game/Core/GameModeDef.UpdateScore` _asgame_mode_def)
          (else
            (`MovementComponent.StopMovementImmediately` (`self.CharacterMovement`))
            (`self.LaunchCharacter` (* (`KismetMathLibrary.Normal` (`self.GetActorForwardVector` (`GameplayStatics.GetPlayerCharacter` 0))) (750.0 750.0 0.0)))
            (`KismetSystemLibrary.Delay` 0.2)))
        (else
          ;;[1 1 1] Fireball
          (if (`GameplayStatics.ObjectIsA` OtherActor "/Game/Projectiles/FireballProjectile_BP.FireballProjectile_BP_C")
            (`self.DeathSound`)
            (`self.K2_DestroyActor`)))))))

(event `self.ReceiveTick`
  (params (DeltaSeconds :type "Float (single-precision)")))

(event `self.PawnSensing.OnSeePawn`
  (params (Pawn :type "Pawn Object Reference"))
  ;[1 1 1] See and Move to Player
  (set `self.isSeeingPlayer` true)
  (`self.FollowPlayer`))

(event `FollowPlayer`
  ;[1 1 1] See and Move to Player
  (if (`self.isSeeingPlayer`)
    (`|AIMoveTo` self (0.0 0.0 0.0) (`GameplayStatics.GetPlayerCharacter` 0))))

(event `DeathSound`
  ;[1 1 1] Death Sound
  (bind _returnvalue (`GameplayStatics.CreateSound2D` "/Game/BigFiles/Audio/Enemy_Death_Sound.Enemy_Death_Sound" 1.0 1.0 0.0 null))
  (`AudioComponent.SetPitchMultiplier` _returnvalue (`self.DeathPitch`))
  (`AudioComponent.Play` _returnvalue 0.0))

(fn `UserConstructionScript`)