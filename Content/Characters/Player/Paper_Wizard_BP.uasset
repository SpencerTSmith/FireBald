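; Player wizard character Blueprint that shows the high score UI and handles taking damage from goblins.
; On BeginPlay it creates the HighScore_BP widget and adds it to the viewport.
; A hit from a Goblin_BP launches the wizard horizontally along the goblin's forward vector and reduces health.
; When health reaches zero or below, it opens the MainMenu level.
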(event `self.ReceiveBeginPlay`
  (bind _returnvalue (`|CreateWidget` "/Game/BigFiles/UI/HighScore_BP.HighScore_BP_C"))
  (`UserWidget.AddToViewport` _returnvalue 0))

(event `self.ReceiveHit`
  (params (MyComp :type "PrimitiveComponent Object Reference") (Other :type "Actor Object Reference") (OtherComp :type "PrimitiveComponent Object Reference") (bSelfMoved :type Boolean) (HitLocation :type "Vector Structure") (HitNormal :type "Vector Structure") (NormalImpulse :type "Vector Structure") (Hit :type "HitResult Structure (by ref)"))
  (if (`GameplayStatics.ObjectIsA` Other "/Game/Characters/Enemy/Goblin_BP.Goblin_BP_C")
    (`self.LaunchCharacter` (* (`self.GetActorForwardVector` Other) (1200.0 1200.0 0.0)))
    (`self.UpdateHealth` -5)
    (if (<= (`self.GetHealth`) 0)
      (`GameplayStatics.OpenLevel` "MainMenu"))))

(fn `UserConstructionScript`)